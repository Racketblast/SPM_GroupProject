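; BP_Flying_AI_Hard is a flying AI enemy, apparently the hard variant, whose graph here handles only audio feedback.
; On BeginPlay it starts its AudioComponent and binds OnEnemyDied to play an explosion sound at that component's location.
; Any damage sets the component's sound to the alien hurt cue and spawns attached copies, capped at two by boolean flags cleared on audio finish.
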(event Custom|OnAudioFinished_Event
  (Variables|Default|SetHurting1 false))

(event Custom|OnAudioFinished_Event_0
  (Variables|Default|SetHurting2 false))

(event Custom|OnEnemyDied_Event
  (params (DeadEnemy :type AI%20Main%20Object%20Reference))
  (Audio|SpawnSoundatLocation "/Game/StarterContent/Audio/Explosion_Cue.Explosion_Cue" (Transformation|GetWorldLocation (Variables|Default|GetAudioComponent)) "0, 0, 0" 1.0 1.0 0.0 0 0))

(event EventBeginPlay
  (EventDispatchers|AssignOnEnemyDied (delegate Custom|OnEnemyDied_Event))
  (Audio|Components|Audio|Play (Variables|Default|GetAudioComponent) 0.0))

(event Game|Damage|EventAnyDamage
  (params (Damage :type Float%20%28single-precision%29) (DamageType :type Damage%20Type%20Object%20Reference) (InstigatedBy :type Controller%20Object%20Reference) (DamageCauser :type Actor%20Object%20Reference))
  (bind _audiocomponent (Variables|Default|GetAudioComponent))
  (Audio|Components|Audio|SetSound _audiocomponent "/Game/Audio/SoundCues/pd_alienHurt_Cue.pd_alienHurt_Cue")
  (if (Variables|Default|GetHurting1)
    (if (not (Variables|Default|GetHurting2))
      (Variables|Default|SetHurting2 true)
      (bind _returnvalue (Audio|SpawnSoundAttached "/Game/Audio/SoundCues/pd_alienHurt_Cue.pd_alienHurt_Cue" _audiocomponent "None" "0, 0, 0" "0, 0, 0" "KeepRelativeOffset" false 1.0 1.0 0.0 0 0))
      (EventDispatchers|AssignOnAudioFinished _returnvalue (delegate Custom|OnAudioFinished_Event_0)))
    (else
      (Variables|Default|SetHurting1 true)
      (bind _returnvalue_2 (Audio|SpawnSoundAttached "/Game/Audio/SoundCues/pd_alienHurt_Cue.pd_alienHurt_Cue" _audiocomponent "None" "0, 0, 0" "0, 0, 0" "KeepRelativeOffset" false 1.0 1.0 0.0 0 0))
      (EventDispatchers|AssignOnAudioFinished _returnvalue_2 (delegate Custom|OnAudioFinished_Event)))))

(fn ConstructionScript)