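; BP_AI_Ranged_Medium is an AI enemy character that hurts the player on contact and can leap to a destination.
; Player overlap sets a collision flag, and Tick uses a 0.25-second Delay to recheck it before applying randomized damage scaled from AIDamage.
; Each hit also notifies the ChallengeSubsystem for challenge tracking.
; JumpToDestination launches the character along a suggested projectile arc aimed above the target point.
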(event EventBeginPlay)

(event EventTick
  (params (DeltaSeconds :type Float%20%28single-precision%29))
  (bind _is_colliding (Variables|Default|GetIs%20Colliding))
  (if _is_colliding
    (Utilities|FlowControl|Delay 0.25)
    (if _is_colliding
      ;[0.02005 0.1105 0.15 0.5] För Challenges, kallar på NotifyPlayerDamaged när spelaren tar skada
      (Class|ChallengeSubsystem|NotifyPlayerDamaged (Subsystems|GetChallengeSubsystem))
      (Game|Damage|ApplyDamage (Game|Player|GetPlayerPawn 0) (Math|Random|RandomFloatinRange (* (Variables|Default|GetAIDamage) 0.3) (Variables|Default|GetAIDamage)) 0 0)
      (else
        (Development|PrintText "Cant catch me")))))

(event Collision|EventActorBeginOverlap
  (params (OtherActor :type Actor%20Object%20Reference))
  (Utilities|Casting|CastToBP_MyPlayerCharacter OtherActor)
  (Variables|Default|SetIs%20Colliding true))

(event Collision|EventActorEndOverlap
  (params (OtherActor :type Actor%20Object%20Reference))
  (Utilities|Casting|CastToBP_MyPlayerCharacter OtherActor)
  (Variables|Default|SetIs%20Colliding false))

(fn ConstructionScript)

(fn JumptoDestination
  (params (Destination :type Vector))
  (bind (_x _y _z) (Math|Vector|BreakVector Destination))
  (bind _outlaunchvelocity (Game|SuggestProjectileVelocityCustomArc (Transformation|GetActorLocation) (Math|Vector|MakeVector _x _y (+ _z 2e+02)) 0.0 0.5))
  (Character|LaunchCharacter _outlaunchvelocity true true))