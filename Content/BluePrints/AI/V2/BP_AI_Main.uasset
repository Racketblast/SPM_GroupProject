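; Alien enemy AI character that voices alien dialogue and can leap to a destination.
; BeginPlay starts an AudioComponent loop that replays after random delays; damage restarts playback, setting the hurt cue variable without reapplying it to the component.
; A second spawned-sound loop with an explosion death branch has no external trigger here, and the death event only prints a debug string.
; JumpToDestination launches the character along a suggested projectile arc aimed above the target.
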(event Custom|OnEnemyDied_Event
  (params (DeadEnemy :type AI%20Main%20Object%20Reference))
  (Development|PrintString "Hello"))

(event Custom|OnAudioFinished_Event
  ;[0.15 0.15 0.15 0.5] Spelar upp generella ljud som Alien gör. OBS! Spelar fortfarande upp vid död
  (Utilities|FlowControl|Delay (Math|Random|RandomFloatinRange 2.0 2.5))
  (Variables|Default|SetAlienDialogue "/Game/Audio/SoundCues/pd_generalAlien_Cue.pd_generalAlien_Cue")
  (if (Variables|Default|GetbIsDead)
    (if (Variables|Default|GetplayedDeathSound)
      (Audio|SpawnSoundAttached "/Game/StarterContent/Audio/Explosion_Cue.Explosion_Cue" 0 "None" "0, 0, 0" "0, 0, 0" "KeepRelativeOffset" false 1.0 1.0 0.0 0 0)
      (Variables|Default|SetplayedDeathSound true))
    (else
      (bind _returnvalue (Audio|SpawnSoundAttached (Variables|Default|GetAlienDialogue) 0 "None" "0, 0, 0" "0, 0, 0" "KeepRelativeOffset" false 1.0 1.0 0.0 0 0))
      (EventDispatchers|AssignOnAudioFinished _returnvalue (delegate Custom|OnAudioFinished_Event)))))

(event Custom|OnAudioFinished_Event_0
  (bind _audiocomponent (Variables|Default|GetAudioComponent))
  (Utilities|FlowControl|Delay (Math|Random|RandomFloatinRange 1.0 2.0))
  (Variables|Default|SetAlienDialogue "/Game/Audio/SoundCues/pd_generalAlien_Cue.pd_generalAlien_Cue")
  (Audio|Components|Audio|Play _audiocomponent 0.0)
  (EventDispatchers|AssignOnAudioFinished _audiocomponent (delegate Custom|OnAudioFinished_Event_0)))

(event EventBeginPlay
  (bind _audiocomponent (Variables|Default|GetAudioComponent))
  (EventDispatchers|AssignOnEnemyDied (delegate Custom|OnEnemyDied_Event))
  (Audio|Components|Audio|SetSound _audiocomponent (Variables|Default|GetAlienDialogue))
  (Audio|Components|Audio|Play _audiocomponent 0.0)
  (EventDispatchers|AssignOnAudioFinished _audiocomponent (delegate Custom|OnAudioFinished_Event_0)))

(event Collision|EventActorBeginOverlap
  (params (OtherActor :type Actor%20Object%20Reference)))

(event Game|Damage|EventAnyDamage
  (params (Damage :type Float%20%28single-precision%29) (DamageType :type Damage%20Type%20Object%20Reference) (InstigatedBy :type Controller%20Object%20Reference) (DamageCauser :type Actor%20Object%20Reference))
  (bind _audiocomponent (Variables|Default|GetAudioComponent))
  (Variables|Default|SetAlienDialogue "/Game/Audio/SoundCues/pd_alienHurt_Cue.pd_alienHurt_Cue")
  (Audio|Components|Audio|Play _audiocomponent 0.0)
  (EventDispatchers|AssignOnAudioFinished _audiocomponent (delegate Custom|OnAudioFinished_Event_0)))

(fn ConstructionScript)

(fn JumptoDestination
  (params (Destination :type Vector))
  (bind (_x _y _z) (Math|Vector|BreakVector Destination))
  (bind _outlaunchvelocity (Game|SuggestProjectileVelocityCustomArc (Transformation|GetActorLocation) (Math|Vector|MakeVector _x _y (+ _z 2e+02)) 0.0 0.5))
  (Character|LaunchCharacter _outlaunchvelocity true true))