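; BP_AI1 is a wave enemy character that takes projectile damage and restarts the player at the Hub level on overlap.
; Sighting the player through PawnSensing sets the HasSeen blackboard key.
; Two projectile types deal different damage; at zero health it destroys itself and notifies BP_WaveManager of the kill.
; Helper functions launch it along an arc to a destination and spawn a BP_MoneyBox, though neither is called here.
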(event OnSeePawn(PawnSensing)
  (params (Pawn :type Pawn%20Object%20Reference))
  (Utilities|Casting|CastToBP_MyPlayerCharacter Pawn)
  (AI|Components|Blackboard|SetValueasBool (AI|GetBlackboard (AI|GetAIController self)) (Utilities|Name|MakeLiteralName "HasSeen") true))

(event Custom|DealDamage_P2
  (Variables|Default|SetAIHealth (- (Variables|Default|GetAIHealth) 50))
  (if (<= (Variables|Default|GetAIHealth) 0)
    (Development|PrintString "AI Dead")
    (Actor|DestroyActor)
    (bind _returnvalue (Actor|GetActorOfClass "/Game/BluePrints/WaveSpawnSystem/BP_WaveManager.BP_WaveManager_C"))
    (bind _asbp_wave_manager (Utilities|Casting|CastToBP_WaveManager _returnvalue))
    (Class|WaveManager|OnEnemyKilled _asbp_wave_manager)))

(event Custom|DealDamage_P1
  (Variables|Default|SetAIHealth (- (Variables|Default|GetAIHealth) 30))
  (if (<= (Variables|Default|GetAIHealth) 0)
    (Development|PrintString "AI Dead")
    (Actor|DestroyActor)
    (bind _returnvalue (Actor|GetActorOfClass "/Game/BluePrints/WaveSpawnSystem/BP_WaveManager.BP_WaveManager_C"))
    (bind _asbp_wave_manager (Utilities|Casting|CastToBP_WaveManager _returnvalue))
    (Class|WaveManager|OnEnemyKilled _asbp_wave_manager)))

(event EventBeginPlay)

(event EventTick
  (params (DeltaSeconds :type Float%20%28single-precision%29)))

(event Collision|EventActorBeginOverlap
  (params (OtherActor :type Actor%20Object%20Reference))
  (Utilities|Casting|CastToBP_Projectile1 OtherActor
    (:then
      (CallFunction|DealDamageP1)
      (Development|PrintString "1 Hit"))
    (:CastFailed
      (Utilities|Casting|CastToBP_Projectile2 OtherActor
        (:then
          (CallFunction|DealDamageP2)
          (Development|PrintString "2 Hit"))
        (:CastFailed
          (Utilities|Casting|CastToBP_MyPlayerCharacter OtherActor)
          (Development|PrintText "Restart")
          (Game|OpenLevel(byName) "Hub"))))))

(fn ConstructionScript)

(fn JumptoDestination
  (params (Destination :type Vector))
  (bind (_x _y _z) (Math|Vector|BreakVector Destination))
  (bind _outlaunchvelocity (Game|SuggestProjectileVelocityCustomArc (Transformation|GetActorLocation) (Math|Vector|MakeVector _x _y (+ _z 2e+02)) 0.0 0.5))
  (Character|LaunchCharacter _outlaunchvelocity true true))

(fn SpawnBuyBox
  (bind _returnvalue (Transformation|GetActorTransform))
  (Game|SpawnActorfromClass "/Game/BluePrints/BP_MoneyBox.BP_MoneyBox_C" (Math|Transform|MakeTransform (Math|Vector|MakeVector (.x (.location _returnvalue)) (.y (.location _returnvalue)) (- (.z (.location _returnvalue)) 5e+01)) (.rotation _returnvalue) (.scale _returnvalue)) "Undefined" "MultiplyWithRoot" 0 0)
  (return))