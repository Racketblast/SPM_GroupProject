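; Behavior tree task that moves the controlled AI pawn to a flanking position around the first player character.
; It offsets the player's location by RadiusPlayer along a randomized horizontal angle, then passes that point through GetRandomReachablePointInRadius to get the destination.
; AI MoveTo runs to that destination, and the task finishes as successful whether the move succeeds or fails.
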(event EventReceiveExecuteAI
  (params (OwnerController :type AI%20Controller%20Object%20Reference) (ControlledPawn :type Pawn%20Object%20Reference))
  (bind _radiusplayer (Variables|Default|GetRadiusPlayer))
  (bind _returnvalue (Game|GetPlayerCharacter 0))
  (bind _returnvalue_2 (Transformation|GetActorLocation _returnvalue))
  (bind _returnvalue_3 (Math|Random|RandomFloatinRange 0.0 3.6e+02))
  (bind _returnvalue_4 (Math|Float|MultiplybyPi _returnvalue_3))
  (AI|AIMoveTo ControlledPawn (.RandomLocation (AI|Navigation|GetRandomReachablePointinRadius (+ _returnvalue_2 (Math|Vector|MakeVector (* (Math|Trig|Cos(Radians) _returnvalue_4) _radiusplayer) (* (Math|Trig|Sin(Radians) _returnvalue_4) _radiusplayer) 0.0)) 0.0 0 0)) 0 1e+02 false
    (:OnSuccess
      _)
    (:OnFail
      _))
  (AI|BehaviorTree|FinishExecute true))