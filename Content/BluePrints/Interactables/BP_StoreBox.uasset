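; BP_StoreBox is an interactable actor whose mesh changes appearance with the game's WeirdMode setting.
; Each Tick it reads WeirdMode from PlayerGameInstance and compares it to a cached value.
; On a change it swaps the static mesh material between the standard top hat currency material and its pink variant.
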(event EventBeginPlay)

(event Collision|EventActorBeginOverlap
  (params (OtherActor :type Actor%20Object%20Reference)))

(event EventTick
  (params (DeltaSeconds :type Float%20%28single-precision%29))
  (bind _asplayer_game_instance (Utilities|Casting|CastToPlayerGameInstance (Game|GetGameInstance)))
  (if (!= (Variables|/Script/SPM_GroupProject.PlayerGameInstance|GetbWeirdMode _asplayer_game_instance) (Variables|Default|GetbCachedWeirdMode))
    (bind _output_get (Variables|Default|SetbCachedWeirdMode (Variables|/Script/SPM_GroupProject.PlayerGameInstance|GetbWeirdMode _asplayer_game_instance)))
    (if _output_get
      (Rendering|Material|SetMaterial (Variables|Default|GetStaticMesh) 0 "/Game/Objects/Materials/Colin/M_TopHatCurrencyPink.M_TopHatCurrencyPink")
      (else
        (Rendering|Material|SetMaterial (Variables|Default|GetStaticMesh) 0 "/Game/Objects/Materials/Colin/M_TopHatCurrency.M_TopHatCurrency")))))

(fn ConstructionScript)