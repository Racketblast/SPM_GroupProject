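; Arena player controller that lets a gamepad drive the mouse cursor while UI is open.
; Each Tick, MoveCursorWithGamePad offsets the mouse position by the left stick scaled by CursorMoveSpeed, with Y inverted.
; It sets the mouse location only when the new position differs beyond a small tolerance, and only while UIOpen is true.
; Gamepad clicking is unfinished: the bottom face button check does nothing and the simulated left-click is disconnected.
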(event EventBeginPlay)

(event EventTick
  (params (DeltaSeconds :type Float%20%28single-precision%29))
  (CallFunction|MoveCursorwithGamePad)
  (if (== (Class|PlayerController|GetInputAnalogKeyState "Gamepad_FaceButton_Bottom") 1.0)
    _))

(fn ConstructionScript)

(fn MoveCursorwithGamePad
  (bind _returnvalue (Game|GetPlayerController 0))
  (bind (_stickx _sticky) (Class|PlayerController|GetInputAnalogStickState "CAS_LeftStick"))
  (bind (_locationx _locationy) (Game|Player|GetMousePosition))
  (bind _cursormovespeed (Variables|Default|GetCursorMoveSpeed))
  (bind (_locationx_2 _locationy_2) (Game|Player|GetMousePosition _returnvalue))
  (bind _returnvalue_2 (* _cursormovespeed _sticky))
  (bind _returnvalue_3 (* _stickx _cursormovespeed))
  (bind _returnvalue_4 (+ _returnvalue_3 _locationx_2))
  (bind _returnvalue_5 (* _returnvalue_2 -1.0))
  (bind _returnvalue_6 (Math|Float|Round _returnvalue_4))
  (bind _returnvalue_7 (+ _returnvalue_5 _locationy_2))
  (bind _returnvalue_8 (Math|Float|Round _returnvalue_7))
  (if (Variables|Default|GetbUIOpen)
    (Variables|Default|SetNewMousePosition (Math|Vector2D|MakeVector2D (Math|Conversions|ToFloat(Integer) _returnvalue_6) (Math|Conversions|ToFloat(Integer) _returnvalue_8)))
    (if (not (Utilities|Operators|EqualEqual (Variables|Default|GetNewMousePosition) (Math|Vector2D|MakeVector2D _locationx _locationy) 1.0))
      (Class|PlayerController|SetMouseLocation (Game|GetPlayerController 0) _returnvalue_6 _returnvalue_8))))